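; Game state that tracks score, lives and enemy phase progression for the current level.
; On BeginPlay it briefly delays, refreshes the HUD, then loads phase thresholds and enemy lists from the DT_Levels row matching the level name.
; Score gains advance phases through BP_GameMode and flag when thresholds run out.
; It also gates player respawns and serves each phase's next enemy class and score using spawn counters.
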(event `self.ReceiveBeginPlay`
  (`KismetSystemLibrary.Delay` 1e-05)
  (`self.SetWidgetScore`)
  (`self.SetWidgetLives`)
  (bind _returnvalue (`GameplayStatics.GetCurrentLevelName` true))
  (bind _outrownames (`DataTableFunctionLibrary.GetDataTableRowNames` "/Game/Table/DT_Levels.DT_Levels"))
  (for _array_element _outrownames
    (bind _returnvalue_2 (`|GetDataTableRow` "/Game/Table/DT_Levels.DT_Levels" _array_element)
      (:`then`
        (bind (_levelname _finalphase _phasewinscore _phaseenemytypes) (break `/Game/Table/F_Level` _returnvalue_2))
        (if (== _levelname _returnvalue)
          (set `self.Final Phase` _finalphase)
          (set `self.Phase Win Score` _phasewinscore)
          (set `self.Phase Enemy Types_0` _phaseenemytypes)
          (break))))))

(fn `CanPlayerRespawn`
  (returns (Success :type Boolean) (CurrentPhase :type Integer))
  (bind _coutlife (`self.CoutLife`))
  (bind _returnvalue (>= _coutlife 0))
  (`/Engine/EditorBlueprintResources/StandardMacros.DecrementInt` _coutlife
    (:`  `
      (if _returnvalue
        (`self.SetWidgetLives`))
      (return _returnvalue (`self.CurrentPhase`)))))

(fn `CheckEnemyForPhase`
  (returns (Valid :type Boolean) (`Phase Enemy Types` :type "Actor Class Reference") (`Score Cout` :type Integer))
  (locals (EnemyInfo :type "/Game/Table/F_EnemySpawnInfo Structure"))
  (bind _phase_enemy_types_0 (`self.Phase Enemy Types_0`))
  (bind _currentphase (`self.CurrentPhase`))
  (bind _enemytypeindex (`self.EnemyTypeIndex`))
  (bind _enemyinfo (break `/Game/Table/F_PhaseEnemy` (`|GetArrayItem` _phase_enemy_types_0 _currentphase)))
  (if (`KismetArrayLibrary.Array_IsValidIndex` _phase_enemy_types_0 _currentphase)
    (if (`KismetArrayLibrary.Array_IsValidIndex` _enemyinfo _enemytypeindex)
      (bind _output_get (set `local.EnemyInfo` (`|GetArrayItem` _enemyinfo _enemytypeindex)))
      (bind (_enemytypeactor _enemycout _scorecout) (break `/Game/Table/F_EnemySpawnInfo` _output_get))
      (if (`KismetSystemLibrary.IsValidClass` _enemytypeactor)
        (bind _returnvalue (< (`self.EnemyCoutIndex`) _enemycout))
        (if _returnvalue
          (return _returnvalue _enemytypeactor _scorecout)
          (else
            (set `self.EnemyCoutIndex` 0)
            (`/Engine/EditorBlueprintResources/StandardMacros.IncrementInt` (`self.EnemyTypeIndex`))))))))

(fn `IncrementEnemy`
  (params (Cout :type Integer))
  (set `self.CurrentCoutEnemy` (+ (`self.CurrentCoutEnemy`) Cout))
  (if (> Cout 0)
    (set `self.EnemyCoutIndex` (+ (`self.EnemyCoutIndex`) 1))))

(fn `IncrementScore`
  (params (ChangeValue :type Integer))
  (returns (bIsWin :type Boolean))
  (bind _currentphase (`self.CurrentPhase`))
  (bind _currentphase_2 (`self.CurrentPhase`))
  (bind _phase_win_score (`self.Phase Win Score`))
  (set `self.Score` (+ ChangeValue (`self.Score`)))
  (`self.SetWidgetScore`)
  (if (`KismetArrayLibrary.Array_IsValidIndex` _phase_win_score _currentphase_2)
    (if (<= (`|GetArrayItem` _phase_win_score _currentphase_2) (`self.Score`))
      (set `self.EnemyTypeIndex` 0)
      (bind _output_get (set `self.CurrentPhase` (+ _currentphase 1)))
      (bind _asbp_game_mode (cast `/Game/BluePrint/Game/BP_GameMode` (`GameplayStatics.GetGameMode`)))
      (`/Game/BluePrint/Game/BP_GameMode.NextPhaseStart` _asbp_game_mode _output_get)
      (if (not (`KismetArrayLibrary.Array_IsValidIndex` (`self.Phase Win Score`) _currentphase))
        (return true)))))

(fn `SetWidgetLives`
  (bind _asbp_player_controller (cast `/Game/BluePrint/Game/BP_PlayerController` (`GameplayStatics.GetPlayerController` 0)))
  (`/Game/BluePrint/Widget/Stats/BPW_Stats.SetLives` (`/Game/BluePrint/Widget/BPW_InGame.BPW_Stats` (`/Game/BluePrint/Game/BP_PlayerController.InGameWidget` _asbp_player_controller)) (`self.CoutLife`)))

(fn `SetWidgetScore`
  (bind _asbp_player_controller (cast `/Game/BluePrint/Game/BP_PlayerController` (`GameplayStatics.GetPlayerController` 0)))
  (`/Game/BluePrint/Widget/Stats/BPW_Stats.SetScore` (`/Game/BluePrint/Widget/BPW_InGame.BPW_Stats` (`/Game/BluePrint/Game/BP_PlayerController.InGameWidget` _asbp_player_controller)) (`self.Score`)))

(fn `UserConstructionScript`)