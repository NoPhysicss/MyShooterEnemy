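; Player controller for the multiplayer lobby that sets up the lobby menu and keeps the selected level name in sync.
; BeginPlay polls until PlayerState is valid, then, for the local player, shows the cursor, views through a level camera and creates BPW_LobbyMenu.
; The host fills level buttons from DT_Levels and reports the first level to BP_LobbyMode.
; Clients display the server's current level, and an event updates the menu's level name.
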(event `self.ReceiveBeginPlay`
  (bind _returnvalue (`GameplayStatics.GetPlayerController` 0))
  (bind _returnvalue_2 (`KismetSystemLibrary.IsServer`))
  (bind _lobbymenu (`self.LobbyMenu`))
  (`/Engine/EditorBlueprintResources/StandardMacros.IsValid` (`self.PlayerState`) :!label _label
    (:`Is Valid`
      (if (`self.IsLocalPlayerController`)
        (set `PlayerController.bShowMouseCursor` true _returnvalue)
        (bind _returnvalue_3 (`GameplayStatics.GetActorOfClass` "/Script/Engine.CameraActor"))
        (`self.SetViewTargetWithBlend` _returnvalue _returnvalue_3 0.0 "VTBlend_Linear" 0.0 false)
        (bind _returnvalue_4 (`|CreateWidget` "/Game/BluePrint/Widget/Menu/LobbyMenu/BPW_LobbyMenu.BPW_LobbyMenu_C" _returnvalue _returnvalue_2 (`PlayerState.GetPlayerName` (`self.PlayerState`))))
        (set `self.LobbyMenu` _returnvalue_4)
        (`UserWidget.AddToViewport` _returnvalue_4 0)
        (if _returnvalue_2
          (bind _outrownames (`DataTableFunctionLibrary.GetDataTableRowNames` "/Game/Table/DT_Levels.DT_Levels"))
          (bind _returnvalue_5 (`|GetDataTableRow` "/Game/Table/DT_Levels.DT_Levels" (`|GetArrayItem` _outrownames))
            (:`then`
              (bind _levelname (break `/Game/Table/F_Level` _returnvalue_5))
              (`/Game/BluePrint/Widget/Menu/LobbyMenu/BPW_LobbyMenu.UpdateLevelName` (`self.LobbyMenu`) _levelname)
              (`self.UpdatePlayerSelectedMap` _levelname)
              (for _array_element _outrownames
                (bind _returnvalue_6 (`|GetDataTableRow` "/Game/Table/DT_Levels.DT_Levels" _array_element)
                  (:`then`
                    (bind _returnvalue_7 (`|CreateWidget` "/Game/BluePrint/Widget/Menu/LobbyMenu/BPW_LobbyLevelButton.BPW_LobbyLevelButton_C" null (`.LevelName_2_B83885714C3F80A0FB99FCA19F3A6547` (break `/Game/Table/F_Level` _returnvalue_6)) _lobbymenu))
                    (`VerticalBox.AddChildToVerticalBox` (`/Game/BluePrint/Widget/Menu/LobbyMenu/BPW_LobbyMenu.SelectLevelByHost` _lobbymenu) _returnvalue_7))
                  (:`RowNotFound`
                    (`KismetSystemLibrary.PrintString` "Check Level Table" true true (struct :`R` 1.0 :`B` 0.070282 :`A` 1.0) :!label _label_2)))))
            (:`RowNotFound`
              (goto _label_2)))
          (else
            (`/Game/BluePrint/Widget/Menu/LobbyMenu/BPW_LobbyMenu.UpdateLevelName` _returnvalue_4 (`self.CurrentLevelByServer`))))))
    (:`Is Not Valid`
      (`KismetSystemLibrary.Delay` 0.01)
      (goto _label))))

(event `UpdateMeReady`)

(event `UpdatePlayerSelectedMap`
  (params (CurentLevelByServer :type Name))
  (bind _asbp_lobby_mode (cast `/Game/BluePrint/Game/Menu/Lobby/BP_LobbyMode` (`GameplayStatics.GetGameMode`)))
  (`/Game/BluePrint/Game/Menu/Lobby/BP_LobbyMode.UpdateLevelName` _asbp_lobby_mode CurentLevelByServer))

(event `UpdateLobbyWidgetOnClient`
  (params (Name :type Name))
  (`/Game/BluePrint/Widget/Menu/LobbyMenu/BPW_LobbyMenu.UpdateLevelName` (`self.LobbyMenu`) Name))

(fn `UserConstructionScript`)