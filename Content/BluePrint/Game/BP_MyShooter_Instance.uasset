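; Game instance Blueprint for the shooter that handles hosting and joining of multiplayer sessions.
; CreateSession stores the max player count, creates a session with optional LAN, then opens LobbyWorld as a listen server.
; JoinSession forwards a search result to the join node, using the first player controller.
; Session failures, network errors and travel errors are only reported through printed messages.
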(event `self.HandleNetworkError`
  (params (FailureType :type "ENetworkFailure Enum" :default "NetDriverAlreadyExists") (bIsServer :type Boolean))
  (`KismetSystemLibrary.PrintString` (`KismetStringLibrary.Concat_StrStr` "NetWork Error - " (`|GetEnumeratorNameAsString` FailureType)) true true (struct :`R` 1.0 :`B` 0.034619 :`A` 1.0)))

(event `self.HandleTravelError`
  (params (FailureType :type "ETravelFailure Enum" :default "NoLevel"))
  (`KismetSystemLibrary.PrintString` (`KismetStringLibrary.Concat_StrStr` "Travle Error - " (`|GetEnumeratorNameAsString` FailureType)) true true (struct :`R` 1.0 :`B` 0.034619 :`A` 1.0)))

(event `/Game/BluePrint/Game/Menu/Lobby/BP_NetworkInterface.CreateSession`
  (params (MaxPlayers :type Integer) (bIsLan :type Boolean))
  (`self.LaunchLobbyEvent` MaxPlayers bIsLan))

(event `LaunchLobbyEvent`
  (params (MaxPlayer :type Integer) (bUseLAN :type Boolean))
  (set `self.MaxPlayer` MaxPlayer)
  (`CreateSessionCallbackProxy.CreateSession` (`GameplayStatics.GetPlayerController` 0) (`self.MaxPlayer`) bUseLAN
    (:`then`
      (`GameplayStatics.OpenLevel` "LobbyWorld" true "Listen"))
    (:`OnFailure`
      (`KismetSystemLibrary.PrintString` "Failed to create Session" true true (struct :`R` 1.0 :`B` 0.167948 :`A` 1.0) 5.0))))

(event `/Game/BluePrint/Game/Menu/Lobby/BP_NetworkInterface.JoinSession`
  (params (SessionToJoin :type "BlueprintSessionResult Structure"))
  (`self.JoinSessionEvent` SessionToJoin))

(event `JoinSessionEvent`
  (params (SearchResult :type "BlueprintSessionResult Structure (by ref)"))
  (`JoinSessionCallbackProxy.JoinSession` (`GameplayStatics.GetPlayerController` 0) SearchResult
    (:`OnFailure`
      (`KismetSystemLibrary.PrintString` "Failed to join Session" true true (struct :`R` 1.0 :`B` 0.167948 :`A` 1.0) 5.0))))