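; Game mode for a phase-based enemy wave game, handling enemy spawning, player respawns and the win screen.
; A looping timer asks BP_GameState for the phase's enemy type and spawns it inside a random phase spawn box, or the boss box for bosses.
; Enemy deaths update GameState count and score, showing BPW_EndGame on a win.
; Respawns use phase-named player starts; phase changes call DestroySelf on living enemies' kill-score components.
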(event `self.ReceiveBeginPlay`
  (`KismetSystemLibrary.K2_SetTimer` null "TryRespawnEnemy" 2.0 true))

(fn `ChoosePlayerStart`
  (params (Player :type "Controller Object Reference"))
  (returns (ReturnValue :type "Actor Object Reference"))
  (return (`self.K2_FindPlayerStart` Player "Phase1")))

(fn `EnemyDead`
  (params (Score :type Integer))
  (bind _asbp_game_state (cast `/Game/BluePrint/Game/BP_GameState` (`GameplayStatics.GetGameState`)))
  (`/Game/BluePrint/Game/BP_GameState.IncrementEnemy` _asbp_game_state -1)
  (bind _biswin (`/Game/BluePrint/Game/BP_GameState.IncrementScore` _asbp_game_state Score))
  (if _biswin
    (bind _returnvalue (`|CreateWidget` "/Game/BluePrint/Widget/BPW_EndGame.BPW_EndGame_C" null true))
    (`UserWidget.AddToViewport` _returnvalue 0)
    (set `PlayerController.bShowMouseCursor` true (`GameplayStatics.GetPlayerController` 0))))

(fn `NextPhaseStart`
  (params (`Current Phase` :type Integer))
  (bind _outactors (`GameplayStatics.GetAllActorsOfClass` "/Game/BluePrint/Enemy/BPEnemy/Common/BP_CharacterEnemy_Base.BP_CharacterEnemy_Base_C"))
  (for _array_element _outactors
    (if (not (`/Game/BluePrint/Enemy/BPEnemy/Common/BP_CharacterEnemy_Base.IsDead` _array_element))
      (`/Game/BluePrint/BP_KillScoreComponente.DestroySelf` (`/Game/BluePrint/Enemy/BPEnemy/Common/BP_CharacterEnemy_Base.BP_KillScoreComponente` _array_element)))))

(fn `TryRespawnEnemy`
  (locals (NewLocalVar :type "Actor Class Reference"))
  (bind _spawnpointboss (`self.SpawnPointBoss`))
  (bind _asbp_game_state (cast `/Game/BluePrint/Game/BP_GameState` (`GameplayStatics.GetGameState`)))
  (bind (_valid _phase_enemy_types _score_cout) (`/Game/BluePrint/Game/BP_GameState.CheckEnemyForPhase` _asbp_game_state))
  (if _valid
    (set `self.Enemy Score` _score_cout)
    (bind _returnvalue (select `int` (`/Game/BluePrint/Game/BP_GameState.CurrentPhase` _asbp_game_state) :`0` (`self.SpawnPointPhase1`) :`1` (`self.SpawnPointPhase2`) :`2` (`self.SpawnPointPhase3`) :`3` (`self.SpawnPointPhase4`) :`4` (`self.SpawnPointPhase5`)))
    (bind _output_get (set `self.CurrentPoint` (`|GetArrayItem` _returnvalue (`KismetMathLibrary.RandomIntegerInRange` 0 (- (`KismetArrayLibrary.Array_Length` _returnvalue) 1)))))
    (if (== _phase_enemy_types "/Game/BluePrint/Enemy/BPEnemy/Boss/BP_CharacterEnemy_Boss.BP_CharacterEnemy_Boss_C")
      (`|SpawnActorFromClass` _phase_enemy_types (`KismetMathLibrary.Conv_VectorToTransform` (`KismetMathLibrary.RandomPointInBoundingBox` (`self.K2_GetActorLocation` _spawnpointboss) (`BoxComponent.BoxExtent` (`/Game/BluePrint/Enemy/BPEnemy/EnemySpawner/BP_EnemySpawn.Box` _spawnpointboss)))) "AdjustIfPossibleButAlwaysSpawn" "MultiplyWithRoot" null null)
      (else
        (`|SpawnActorFromClass` _phase_enemy_types (`KismetMathLibrary.Conv_VectorToTransform` (`KismetMathLibrary.RandomPointInBoundingBox` (`self.K2_GetActorLocation` _output_get) (`BoxComponent.BoxExtent` (`/Game/BluePrint/Enemy/BPEnemy/EnemySpawner/BP_EnemySpawn.Box` _output_get)))) "AdjustIfPossibleButAlwaysSpawn" "MultiplyWithRoot" null null)))
    (`/Game/BluePrint/Game/BP_GameState.IncrementEnemy` _asbp_game_state 1)))

(fn `TryToRespawnPlayer`
  (returns (Success :type Boolean))
  (bind _returnvalue (`GameplayStatics.GetPlayerController` 0))
  (`KismetSystemLibrary.PrintString` (`KismetSystemLibrary.GetDisplayName` null))
  (bind _asbp_game_state (cast `/Game/BluePrint/Game/BP_GameState` (`GameplayStatics.GetGameState`)))
  (bind (_success _currentphase) (`/Game/BluePrint/Game/BP_GameState.CanPlayerRespawn` _asbp_game_state))
  (if _success
    (`self.RestartPlayerAtPlayerStart` _returnvalue (`self.K2_FindPlayerStart` _returnvalue (select `int` _currentphase :`0` "Phase0" :`1` "Phase1" :`2` "Phase2" :`3` "Phase3" :`4` "Phase4")))
    (return true)
    (else
      (return _success))))

(fn `UserConstructionScript`)

(fn `WinCondition`)