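; Player controller that sets up the in-game HUD and audio for the player.
; On BeginPlay it pushes the main sound mix and creates the in-game widget, whose health bar is reinitialized on possess and unpossess.
; Each tick while IsAlive is true, it overrides the audio listener to a fixed offset from the player pawn with zero rotation, decoupling hearing from the camera.
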(event `self.ReceiveBeginPlay`
  (`GameplayStatics.PushSoundMixModifier` "/Game/BluePrint/Sounds/MIX_Main.MIX_Main")
  (bind _returnvalue (`|CreateWidget` "/Game/BluePrint/Widget/BPW_InGame.BPW_InGame_C" self))
  (set `self.InGameWidget` _returnvalue)
  (`UserWidget.AddToViewport` _returnvalue 0))

(event `self.ReceiveTick`
  (params (DeltaSeconds :type "Float (single-precision)"))
  (bind _returnvalue (`GameplayStatics.GetPlayerPawn` 0))
  (`/Engine/EditorBlueprintResources/StandardMacros.IsValid` _returnvalue
    (:`Is Valid`
      (if (`self.IsAlive`)
        (`self.SetAudioListenerOverride` null (+ (`self.K2_GetActorLocation` _returnvalue) (-125.0 0.0 125.0)))))))

(event `self.ReceiveUnPossess`
  (params (UnpossessedPawn :type "Pawn Object Reference"))
  (bind _ingamewidget (`self.InGameWidget`))
  (`/Engine/EditorBlueprintResources/StandardMacros.IsValid` _ingamewidget
    (:`Is Valid`
      (`/Game/BluePrint/Widget/Health/BPW_CharStatsBar.InitWidget` (`/Game/BluePrint/Widget/BPW_InGame.HealthBar` _ingamewidget)))))

(event `self.ReceivePossess`
  (params (PossessedPawn :type "Pawn Object Reference"))
  (bind _ingamewidget (`self.InGameWidget`))
  (`/Engine/EditorBlueprintResources/StandardMacros.IsValid` _ingamewidget
    (:`Is Valid`
      (`/Game/BluePrint/Widget/Health/BPW_CharStatsBar.InitWidget` (`/Game/BluePrint/Widget/BPW_InGame.HealthBar` _ingamewidget)))))

(fn `UserConstructionScript`)