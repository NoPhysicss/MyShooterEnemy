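; BP_KillScoreComponente is an actor component that awards a kill score when its owning enemy dies.
; On BeginPlay it binds an event to OnDead on the owner's MyShooterHealthComponent.
; DeadOvner passes Score to BP_GameMode's EnemyDead, then destroys the component.
; A separate DestroySelf event removes the component without reporting a score.
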(event `self.ReceiveBeginPlay`
  (add `MyShooterHealthComponent.OnDead` (`Actor.K2_GetComponentsByClass` (`self.GetOwner`) "/Script/MyShooter.MyShooterHealthComponent") (`|CreateDelegate` :!event `DeadOvner`)))

(event `DeadOvner`
  (bind _asbp_game_mode (cast `/Game/BluePrint/Game/BP_GameMode` (`GameplayStatics.GetGameMode`)))
  (`/Game/BluePrint/Game/BP_GameMode.EnemyDead` _asbp_game_mode (`self.Score`))
  (`self.K2_DestroyComponent`))

(event `DestroySelf`
  (`self.K2_DestroyComponent`))