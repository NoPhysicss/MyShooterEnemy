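; Base pickup actor that passes an overlapping MyShooterCharacter's inventory component to OverlapChatacter, an empty event here.
; InitActor configures it from weapon drop info, keeping either a static or skeletal mesh, destroying the other component and storing the item info.
; PickUpSuccess destroys the actor, while ReSpawnActor hides both meshes and disables sphere collision, then restores them after RespawnTimer.
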(event `OverlapChatacter`
  (params (ToInventory :type "MyInventoryComponent Object Reference")))

(event `self.Sphere.OnComponentBeginOverlap`
  (params (OverlappedComponent :type "PrimitiveComponent Object Reference") (OtherActor :type "Actor Object Reference") (OtherComp :type "PrimitiveComponent Object Reference") (OtherBodyIndex :type Integer) (bFromSweep :type Boolean) (SweepResult :type "HitResult Structure (by ref)"))
  (bind _asmy_shooter_character (cast `MyShooterCharacter` OtherActor))
  (`self.OverlapChatacter` (`MyShooterCharacter.InventoryComponent` _asmy_shooter_character)))

(event `ReSpawnActor`
  (`PrimitiveComponent.SetCollisionEnabled` (`self.Sphere`) "NoCollision")
  (`SceneComponent.SetVisibility` (`self.SkeletalMesh`) false false)
  (`SceneComponent.SetVisibility` (`self.StaticMesh`) false false)
  (`KismetSystemLibrary.Delay` (`self.RespawnTimer`))
  (`SceneComponent.SetVisibility` (`self.StaticMesh`) true false)
  (`SceneComponent.SetVisibility` (`self.SkeletalMesh`) true false)
  (`PrimitiveComponent.SetCollisionEnabled` (`self.Sphere`) "QueryOnly"))

(fn `InitActor`
  (params (`Info Actor` :type "DropItem Structure"))
  (bind (_weaponstaticmesh _weaponskeletmesh _weaponinfo) (break `DropItem` `Info Actor`))
  (`/Engine/EditorBlueprintResources/StandardMacros.IsValid` _weaponstaticmesh
    (:`Is Valid`
      (`ActorComponent.K2_DestroyComponent` (`self.SkeletalMesh`))
      (`StaticMeshComponent.SetStaticMesh` (`self.StaticMesh`) _weaponstaticmesh)
      (set `self.DropItemInfo` _weaponinfo :!label _label)
      (set `self.Have Widget` false)
      (set `self.NewDropInfo` false))
    (:`Is Not Valid`
      (`/Engine/EditorBlueprintResources/StandardMacros.IsValid` _weaponskeletmesh
        (:`Is Valid`
          (`ActorComponent.K2_DestroyComponent` (`self.StaticMesh`))
          (`SkeletalMeshComponent.SetSkeletalMeshAsset` (`self.SkeletalMesh`) _weaponskeletmesh)
          (goto _label))
        (:`Is Not Valid`
          (`KismetSystemLibrary.PrintString` "Error, Actor has no ANY mash"))))))

(fn `PickUpSuccess`
  (`self.K2_DestroyActor`))

(fn `UserConstructionScript`)