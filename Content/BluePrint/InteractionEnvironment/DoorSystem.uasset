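; DoorSystem is a sliding door that moves vertically for the top-down player character.
; Overlapping the enter collision plays a timeline that maps its offset onto the door's relative Z, up to a Z variable.
; Ending overlap with the exit collision reverses the timeline from its end to close the door.
; An open-state flag prevents repeated triggers, and other actors are ignored.
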(event `self.EnterCollision.OnComponentBeginOverlap`
  (params (OverlappedComponent :type "PrimitiveComponent Object Reference") (OtherActor :type "Actor Object Reference") (OtherComp :type "PrimitiveComponent Object Reference") (OtherBodyIndex :type Integer) (bFromSweep :type Boolean) (SweepResult :type "HitResult Structure (by ref)"))
  (cast `/Game/BluePrint/Charecter/BP_TopDownCharacter` OtherActor)
  (if (not (`self.bDoorIsOpen`))
    (set `self.bDoorIsOpen` true)
    (bind (_direction _zoffset) (`Timeline|DoorOpening` :!via `PlayFromStart` :!label _label)
      (:`Update`
        (`SceneComponent.K2_SetRelativeLocation` (`self.Door`) (`KismetMathLibrary.MakeVector` 0.0 0.0 (`KismetMathLibrary.MapRangeClamped` _zoffset 0.0 1.0 0.0 (`self.z`))) false false)))))

(event `self.ExitCollision.OnComponentEndOverlap`
  (params (OverlappedComponent :type "PrimitiveComponent Object Reference") (OtherActor :type "Actor Object Reference") (OtherComp :type "PrimitiveComponent Object Reference") (OtherBodyIndex :type Integer))
  (cast `/Game/BluePrint/Charecter/BP_TopDownCharacter` OtherActor)
  (if (`self.bDoorIsOpen`)
    (set `self.bDoorIsOpen` false)
    (goto _label :!via `ReverseFromEnd`)))

(fn `UserConstructionScript`)