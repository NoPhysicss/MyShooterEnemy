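; Med-aid pickup actor that heals the shooter character who overlaps it.
; It extends the parent's overlap event, casting the inventory's owner to MyShooterCharacter and comparing current to maximum health on its health component.
; Only when health is below maximum, it applies its configured health amount, then either calls the respawn function or completes the pickup, depending on the ReSpawn flag.
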(event `self.ReceiveTick`
  (params (DeltaSeconds :type "Float (single-precision)"))
  (`parent.ReceiveTick` DeltaSeconds))

(event `self.OverlapChatacter`
  (params (ToInventory :type "MyInventoryComponent Object Reference"))
  (`parent.OverlapChatacter` ToInventory)
  (bind _asmy_shooter_character (cast `MyShooterCharacter` (`ActorComponent.GetOwner` ToInventory)))
  (bind _charhealthcomponent (`MyShooterCharacter.CharHealthComponent` _asmy_shooter_character))
  (bind _returnvalue (`MyShooterHealthComponent.GetMaxHealt` _charhealthcomponent))
  (bind _returnvalue_2 (`MyShooterHealthComponent.GetCurrentHealt` _charhealthcomponent))
  (if (< _returnvalue_2 _returnvalue)
    (`MyShooterHealthComponent.ChangeCurrentHealt` _charhealthcomponent (`self.HealthCout`))
    (if (`self.ReSpawn`)
      (`self.ReSpawnActor`)
      (else
        (`self.PickUpSuccess`)))))

(fn `UserConstructionScript`
  (`parent.UserConstructionScript`))