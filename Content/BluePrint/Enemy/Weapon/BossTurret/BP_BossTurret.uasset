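; BP_BossTurret is a boss rocket turret enemy that yaws one bone toward the player every tick.
; A looping timer plays the Shoot timeline, whose event spawns a BP_BossTurretMissle at the rocket socket with explosive projectile info.
; Damage reduces its MyShooterHealth, spawning a floating damage-number actor on each survived hit, or exploding and destroying the turret at zero health.
; Aiming and the initial tilt set PoseableMesh bones directly, resolved from socket names.
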(event `self.ReceiveBeginPlay`
  (`PoseableMeshComponent.SetBoneRotationByName` (`self.PoseableMesh`) (`SkinnedMeshComponent.GetSocketBoneName` (`self.PoseableMesh`) "RotationSocked") (struct :`Roll` 70.0) "WorldSpace")
  (`KismetSystemLibrary.K2_SetTimerDelegate` (delegate `FireEvent`) 5.0 true))

(event `FireEvent`
  (`Timeline|Shoot` :!via `PlayFromStart`
    (:`ShootTiming`
      (`GameplayStatics.PlaySoundAtLocation` "/Game/MilitaryWeapDark/Sound/RocketLauncher/RocketLauncherB_Fire_Cue.RocketLauncherB_Fire_Cue" (`self.K2_GetActorLocation`) (struct) 1.0 1.0 0.0 null null null null)
      (bind _returnvalue (`|SpawnActorFromClass` "/Game/BluePrint/Enemy/Weapon/BossTurret/BP_BossTurretMissle.BP_BossTurretMissle_C" (`KismetMathLibrary.MakeTransform` (.location (`SceneComponent.GetSocketTransform` (`self.PoseableMesh`) "RocketSocket" "RTS_World")) (.rotation (`SceneComponent.GetSocketTransform` (`self.PoseableMesh`) "RocketSocket" "RTS_World"))) "Undefined" "MultiplyWithRoot" self null))
      (`ProjectileDefault.InitProjectile` _returnvalue (make `ProjectileInfo` :`Projectile` "/Game/BluePrint/Enemy/Weapon/BossTurret/BP_BossTurretMissle.BP_BossTurretMissle_C" :`ProjectileDamage` 1.0 :`ProjectileInitSpeed` 500.0 :`ProjectileMaxSpeed` 1500.0 :`ProjectileMinDamage` 1.0 :`DamageReductionDistance` 0.0 :`DamageReductionPerSecondByPersent` 0.0 :`ExploseMaxDamage` 50.0 :`ExploseSound` "/Game/MilitaryWeapDark/Sound/GrenadeLauncher/GrenadeLauncher_Explosion_Cue.GrenadeLauncher_Explosion_Cue" :`ExploseFX` "/Game/MilitaryWeapDark/FX/P_Grenade_Explosion_01.P_Grenade_Explosion_01")))))

(event `self.ReceiveTick`
  (params (DeltaSeconds :type "Float (single-precision)"))
  (bind _returnvalue (`GameplayStatics.GetPlayerPawn` 0))
  (bind (_returnvalue_roll _returnvalue_pitch _returnvalue_yaw) (`KismetMathLibrary.BreakRotator` (`KismetMathLibrary.FindLookAtRotation` (`self.K2_GetActorLocation`) (`self.K2_GetActorLocation` _returnvalue))))
  (`/Engine/EditorBlueprintResources/StandardMacros.IsValid` _returnvalue
    (:`Is Valid`
      (`PoseableMeshComponent.SetBoneRotationByName` (`self.PoseableMesh`) (`SkinnedMeshComponent.GetSocketBoneName` (`self.PoseableMesh`) "RotationToPlayerSocket") (`KismetMathLibrary.MakeRotator` 0.0 0.0 _returnvalue_yaw) "WorldSpace"))))

(event `self.ReceiveAnyDamage`
  (params (Damage :type "Float (single-precision)") (DamageType :type "DamageType Object Reference") (InstigatedBy :type "Controller Object Reference") (DamageCauser :type "Actor Object Reference"))
  (bind _returnvalue (`self.K2_GetActorLocation`))
  (bind _returnvalue_2 (* Damage -1.0))
  (`MyShooterHealthComponent.ChangeCurrentHealt` (`self.MyShooterHealth`) _returnvalue_2)
  (bind _returnvalue_3 (`MyShooterHealthComponent.GetCurrentHealt` (`self.MyShooterHealth`)))
  (if (<= _returnvalue_3 0.0)
    (`GameplayStatics.SpawnEmitterAtLocation` "/Game/FX_Effect/Particles/P_Explosion.P_Explosion" _returnvalue)
    (`GameplayStatics.SpawnSoundAtLocation` "/Game/MilitaryWeapDark/Sound/RocketLauncher/RocketLauncher_Explosion_Cue.RocketLauncher_Explosion_Cue" _returnvalue (struct) 1.0 1.0 0.0 null null)
    (`self.K2_DestroyActor`)
    (else
      (bind _returnvalue_4 (`|SpawnActorFromClass` "/Game/BluePrint/InteractionEnvironment/DamageWidget/DisplayDamageActor.DisplayDamageActor_C" (`KismetMathLibrary.MakeTransform` (+ (`self.K2_GetActorLocation`) (+ (`KismetMathLibrary.MakeVector` (`KismetMathLibrary.RandomFloatInRange` -10.0 10.0) (`KismetMathLibrary.RandomFloatInRange` -10.0 10.0)) (`self.Local Point Spawn Health Number`))) (struct :`Yaw` 180.0)) "Undefined" "MultiplyWithRoot" null null))
      (`/Game/BluePrint/InteractionEnvironment/DamageWidget/DisplayDamageActor.InitActor` _returnvalue_4 _returnvalue_2 _returnvalue_3))))

(fn `UserConstructionScript`)