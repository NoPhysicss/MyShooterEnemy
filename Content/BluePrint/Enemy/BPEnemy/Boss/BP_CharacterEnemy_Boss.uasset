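; Boss enemy character that regenerates health and summons turrets as it weakens.
; Looping timers started on BeginPlay appear to drive both behaviors, with Tick disabled.
; Regeneration adds fixed health below one third of maximum and spawns a floating number actor.
; Turrets spawn at random reachable nearby points in two flag-gated waves at falling health thresholds, after which the turret timer is cleared.
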(event `self.ReceiveBeginPlay`
  (`parent.ReceiveBeginPlay`)
  (`KismetSystemLibrary.K2_SetTimerDelegate` (`|CreateDelegate` :!event `BossRegeneration`) 3.0 true)
  (bind _returnvalue (`KismetSystemLibrary.K2_SetTimerDelegate` (`|CreateDelegate` :!event `BossTurretSpawn`) 5.0 true))
  (set `self.BossTurretTimerHandel` _returnvalue)
  (bind _returnvalue_2 (`MyShooterHealthComponent.GetMaxHealt` (`self.MyShooterHealth`)))
  (set `self.BossMaxHealth` _returnvalue_2))

(event `/Game/BluePrint/Enemy/BPEnemy/Common/BPI_Combat.PawnRangeAttack`
  (`parent.PawnRangeAttack`))

(event `BossRegeneration`
  (bind _myshooterhealth (`self.MyShooterHealth`))
  (bind _returnvalue (`MyShooterHealthComponent.GetCurrentHealt` _myshooterhealth))
  (bind _returnvalue_2 (`MyShooterHealthComponent.GetMaxHealt` _myshooterhealth))
  (if (< _returnvalue (/ _returnvalue_2 3.0))
    (`MyShooterHealthComponent.SetCurrentHealt` (`self.MyShooterHealth`) (+ _returnvalue 100.0))
    (bind _returnvalue_3 (`|SpawnActorFromClass` "/Game/BluePrint/InteractionEnvironment/DamageWidget/DisplayDamageActor.DisplayDamageActor_C" (`KismetMathLibrary.MakeTransform` (+ (`self.K2_GetActorLocation`) (+ (`KismetMathLibrary.MakeVector` (`KismetMathLibrary.RandomFloatInRange` -10.0 10.0) (`KismetMathLibrary.RandomFloatInRange` -10.0 10.0)) (`self.Local Point Spawn Health Number`))) (struct :`Yaw` 180.0)) "Undefined" "MultiplyWithRoot" null null))
    (`/Game/BluePrint/InteractionEnvironment/DamageWidget/DisplayDamageActor.InitActor` _returnvalue_3 100.0 _returnvalue)))

(event `BossTurretSpawn`
  (bind _returnvalue (`MyShooterHealthComponent.GetCurrentHealt` (`self.MyShooterHealth`)))
  (if (< _returnvalue (/ (`self.BossMaxHealth`) 1.4))
    (if (`self.bIsFirstSpawn`)
      (if (< _returnvalue (/ (`self.BossMaxHealth`) 3.0))
        (if (not (`self.bIsSecondSpawn`))
          (set `self.bIsSecondSpawn` true)
          (for _ (range 2)
            (`|SpawnActorFromClass` "/Game/BluePrint/Enemy/Weapon/BossTurret/BP_BossTurret.BP_BossTurret_C" (`KismetMathLibrary.MakeTransform` (`NavigationSystemV1.K2_GetRandomReachablePointInRadius` (`self.K2_GetActorLocation`) 1000.0 null null)) "AdjustIfPossibleButAlwaysSpawn" "MultiplyWithRoot" null null))
          (`KismetSystemLibrary.K2_ClearAndInvalidateTimerHandle` (`self.BossTurretTimerHandel`))))
      (else
        (`|SpawnActorFromClass` "/Game/BluePrint/Enemy/Weapon/BossTurret/BP_BossTurret.BP_BossTurret_C" (`KismetMathLibrary.MakeTransform` (`NavigationSystemV1.K2_GetRandomReachablePointInRadius` (`self.K2_GetActorLocation`) 1000.0 null null)) "AdjustIfPossibleButAlwaysSpawn" "MultiplyWithRoot" null null)
        (set `self.bIsFirstSpawn` true)))))

(fn `UserConstructionScript`
  (`parent.UserConstructionScript`))