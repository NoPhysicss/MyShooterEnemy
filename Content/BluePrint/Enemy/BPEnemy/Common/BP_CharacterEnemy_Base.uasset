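; Base enemy character with ranged and melee montage attacks, a socket-attached weapon and a game-mode-assigned kill score.
; Damage feeds the health component, whose changes spawn damage numbers and roll for stun, hit reaction or temporary slowdown.
; Ranged attacks use the weapon with ammo and reloads, while melee sphere-traces on an anim notify to damage the player.
; Death unpossesses, ragdolls and releases any randomized ammo drop rolled at BeginPlay.
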(event `self.ReceiveBeginPlay`
  (bind _mesh (`self.Mesh`))
  ;[1 1 1] BeginPlay
  (`self.InitDropComponente`)
  (bind _asbp_game_mode (cast `/Game/BluePrint/Game/BP_GameMode` (`GameplayStatics.GetGameMode`)))
  (set `/Game/BluePrint/BP_KillScoreComponente.Score` (`/Game/BluePrint/Game/BP_GameMode.Enemy Score` _asbp_game_mode) (`self.BP_KillScoreComponente`))
  ;[1 1 1] WeponInit
  (bind _returnvalue (`|SpawnActorFromClass` (`self.WeaponActor`) (`KismetMathLibrary.Conv_VectorToTransform` (`SceneComponent.GetSocketLocation` _mesh "WeaponSocket")) "AlwaysSpawn" "MultiplyWithRoot" self null))
  (set `self.Weapon` _returnvalue)
  (`SceneComponent.K2_AttachToComponent` (`Actor.RootComponent` _returnvalue) _mesh "WeaponSocket" "SnapToTarget" "SnapToTarget" "SnapToTarget" true)
  (set `self.AmmoCoutInRifle` (`self.AmmoCout`)))

(event `self.ReceiveTick`
  (params (DeltaSeconds :type "Float (single-precision)"))
  (bind _charactermovement (`self.CharacterMovement`))
  ;[1 1 1] Tick with movement
  (set `self.DeltaTime` DeltaSeconds)
  (if (`self.SlowDownSpeed`)
    (set `CharacterMovementComponent.MaxWalkSpeed` (`KismetMathLibrary.FInterpTo` (`self.Max Walk Speed`) (`self.Min(of Max)Walk Speed`) (`self.DeltaTime`) (`self.SpeedUpInTick`)) _charactermovement)
    (else
      (set `CharacterMovementComponent.MaxWalkSpeed` (`self.Max Walk Speed`) _charactermovement))))

(event `self.ReceiveAnyDamage`
  (params (Damage :type "Float (single-precision)") (DamageType :type "DamageType Object Reference") (InstigatedBy :type "Controller Object Reference") (DamageCauser :type "Actor Object Reference"))
  ;[1 1 1] Enemy Take Damaga
  (`MyShooterHealthComponent.ChangeCurrentHealt` (`self.MyShooterHealth`) (* Damage -1.0)))

(event `self.MyShooterHealth.OnHealthChange`
  (params (Health :type "Float (single-precision)") (Damage :type "Float (single-precision)"))
  ;[1 1 1] Enemy Health
  (if (not (`self.IsDead`))
    (if (> (`self.StunChance`) (`KismetMathLibrary.RandomFloat`))
      (`self.Confusiont Enabled`)
      (else
        (`self.Hit Enabled`)))
    (bind _returnvalue (`|SpawnActorFromClass` "/Game/BluePrint/InteractionEnvironment/DamageWidget/DisplayDamageActor.DisplayDamageActor_C" (`KismetMathLibrary.MakeTransform` (+ (`self.K2_GetActorLocation`) (+ (`KismetMathLibrary.MakeVector` (`KismetMathLibrary.RandomFloatInRange` -10.0 10.0) (`KismetMathLibrary.RandomFloatInRange` -10.0 10.0)) (`self.Local Point Spawn Health Number`))) (struct :`Yaw` 180.0)) "Undefined" "MultiplyWithRoot" null null))
    (`/Game/BluePrint/InteractionEnvironment/DamageWidget/DisplayDamageActor.InitActor` _returnvalue Damage Health)
    (if (`self.CanBeStun`)
      (if (> (`self.SlowDownSpeedChande`) (`KismetMathLibrary.RandomFloat`))
        (set `self.SlowDownSpeed` true)
        (`KismetSystemLibrary.K2_SetTimerDelegate` (delegate `SlowDownSpeedTimer`) (`self.SlownesTime`))))))

(event `SlowDownSpeedTimer`
  ;[1 1 1] Enemy Health
  (set `self.SlowDownSpeed` false))

(event `self.MyShooterHealth.OnDead`
  (bind _deathanims (`self.DeathAnims`))
  (bind _mesh (`self.Mesh`))
  (bind _capsulecomponent (`self.CapsuleComponent`))
  (bind _dropcomponente (`self.DropComponente`))
  (bind _output (`|GetArrayItem` _deathanims (- (`KismetArrayLibrary.Array_Length` _deathanims) 1)))
  ;[1 1 1] Enemy Dead Event
  (if (not (`self.IsDead`))
    (`self.DeadEvent`)
    (`/Engine/EditorBlueprintResources/StandardMacros.IsValid` _output
      (:`Is Valid`
        (`|PlayMontage` (`self.Mesh`) _output
          (:`then`
            _)
          (:`OnInterrupted`
            _))
        (`PrimitiveComponent.SetCollisionEnabled` _mesh "PhysicsOnly")
        (`PrimitiveComponent.SetCollisionResponseToChannel` _capsulecomponent "ECC_PhysicsBody" "ECR_Ignore")
        (`PrimitiveComponent.SetCollisionResponseToChannel` (`self.Mesh`) "ECC_PhysicsBody" "ECR_Ignore")
        (`PrimitiveComponent.SetCollisionResponseToChannel` _capsulecomponent "ECC_Pawn" "ECR_Ignore")
        (`PrimitiveComponent.SetCollisionResponseToChannel` (`self.Mesh`) "ECC_Pawn" "ECR_Ignore")
        (`PrimitiveComponent.SetCollisionResponseToChannel` _capsulecomponent "ECC_WorldDynamic" "ECR_Ignore")
        (`PrimitiveComponent.SetCollisionResponseToChannel` (`self.Mesh`) "ECC_WorldDynamic" "ECR_Ignore")
        (`PrimitiveComponent.SetCollisionResponseToChannel` _capsulecomponent "ECC_GameTraceChannel4" "ECR_Ignore")
        (`PrimitiveComponent.SetCollisionResponseToChannel` (`self.Mesh`) "ECC_GameTraceChannel4" "ECR_Ignore")
        (`PrimitiveComponent.SetCollisionProfileName` _mesh "PhysicsActor" false)
        (`PrimitiveComponent.SetSimulatePhysics` _mesh true)
        (`/Engine/EditorBlueprintResources/StandardMacros.IsValid` _dropcomponente
          (:`Is Valid`
            (`/Game/BluePrint/BP_DropActorComponente.Drop` _dropcomponente)))))))

(event `/Game/BluePrint/Enemy/BPEnemy/Common/BPI_Combat.PawnRangeAttack`
  (bind _rangeattackanims (`self.RangeAttackAnims`))
  (bind _reloadinganims (`self.ReloadingAnims`))
  (if (not (`self.bIsShooting`))
    (`KismetSystemLibrary.Delay` (/ 1.0 (/ (`self.RangetAttackSpeed`) 60.0)))
    (if (== (`self.AmmoCoutInRifle`) 0)
      (if (not (`self.bIsReloading`))
        (set `self.bIsReloading` true)
        (`|PlayMontage` (`self.Mesh`) (`|GetArrayItem` _reloadinganims (`KismetMathLibrary.RandomInteger` (`KismetArrayLibrary.Array_Length` _reloadinganims)))
          (:`OnCompleted`
            (set `self.AmmoCoutInRifle` (`self.AmmoCout`))
            (set `self.bIsReloading` false))))
      (else
        (set `self.bIsShooting` true)
        (`self.SetAttackState` false)
        (`|PlayMontage` (`self.Mesh`) (`|GetArrayItem` _rangeattackanims (`KismetMathLibrary.RandomInteger` (`KismetArrayLibrary.Array_Length` _rangeattackanims)))
          (:`then`
            (`/Game/BluePrint/Enemy/Weapon/BP_EnemyWeapon_Deafault.Fire` (`self.Weapon`))
            (`self.SetAttackState` true)
            (set `self.bIsShooting` false)
            (set `self.AmmoCoutInRifle` (- (`self.AmmoCoutInRifle`) 1))))))))

(event `/Game/BluePrint/Enemy/BPEnemy/Common/BPI_Combat.PawnMeleeAttack`
  (bind _meleeattackanims (`self.MeleeAttackAnims`))
  (bind _basemeleedamage (`self.BaseMeleeDamage`))
  (if (not (`self.bIsReloading`))
    (`self.SetStateMovement` false)
    (`self.SetAttackState` false)
    (bind _notifyname (`|PlayMontage` (`self.Mesh`) (`|GetArrayItem` _meleeattackanims (`KismetMathLibrary.RandomInteger` (`KismetArrayLibrary.Array_Length` _meleeattackanims))))
      (:`OnCompleted`
        (`self.SetStateMovement` true :!label _label)
        (`self.SetAttackState` true))
      (:`OnInterrupted`
        (goto _label))
      (:`OnNotifyBegin`
        (if (== _notifyname "Attack")
          (`self.MeleeAttack` (`self.MeleeAttackStartPoint`) (`self.MeleeAttacklenght`) (`KismetMathLibrary.RandomFloatInRange` (+ _basemeleedamage 25.0) (- _basemeleedamage 10.0)) (`self.MeleeAttackRadius`)))))))

(fn `Confusiont Disabled Timer`
  (`self.SetStateMovement` true)
  (set `CharacterMovementComponent.MaxWalkSpeed` (`self.Max Walk Speed`) (`self.CharacterMovement`))
  (set `self.bIsConfused` false))

(fn `Confusiont Enabled`
  (locals (CurrentMontage :type "AnimMontage Object Reference"))
  (bind _stunanims (`self.StunAnims`))
  (`self.SetStateMovement` false)
  (bind _output_get (set `local.CurrentMontage` (`|GetArrayItem` _stunanims (`KismetMathLibrary.RandomIntegerInRange` 0 (- (`KismetArrayLibrary.Array_Length` _stunanims) 1)))))
  (`KismetSystemLibrary.K2_SetTimer` null "Confusiont Disabled Timer" (`AnimationAsset.GetPlayLength` _output_get))
  (`self.PlayAnimMontage` (`local.CurrentMontage`))
  (set `CharacterMovementComponent.MaxWalkSpeed` 0.0 (`self.CharacterMovement`))
  (set `self.bIsConfused` true))

(fn `DeadEvent`
  (`Controller.UnPossess` (`self.GetController`))
  (`self.SetLifeSpan` 10.0)
  (`self.SetStateMovement` false)
  (`self.SetAttackState` false)
  (set `self.IsDead` true))

(fn `Hit Enabled`
  (locals (HitAnimChance :type "Float (double-precision)" :default 0.2) (HitAnims :type "Array of AnimMontage Object Reference"))
  (bind _hitanims (`local.HitAnims`))
  (if (`self.bIsConfused`)
    _
    (elif (> (`KismetMathLibrary.RandomFloat`) (`local.HitAnimChance`))
      (`self.PlayAnimMontage` (`|GetArrayItem` _hitanims (`KismetMathLibrary.RandomIntegerInRange` 0 (- (`KismetArrayLibrary.Array_Length` _hitanims) 1)))))))

(fn `InitDropComponente`
  (locals (CoutAmmo :type Integer :default 1))
  (if (< (`KismetMathLibrary.RandomFloat`) (`self.AmmoDropChance`))
    (bind _returnvalue (`AddComponent|NODE_AddBP_DropActorComponente-0`))
    (set `self.DropComponente` _returnvalue)
    (bind _output_get (set `/Game/BluePrint/BP_DropActorComponente.Type` (select `int` (`KismetMathLibrary.RandomIntegerInRange` 0 3) :`0` "RifleType" :`1` "ShotGunType" :`2` "SniperRifle" :`3` "GrenadeLauncher" :!type "EWeaponType Enum") _returnvalue))
    (`|ExecutionSequence`
      (:`then_0`
        (switch `EWeaponType` _output_get
          (:`RifleType`
            (set `local.CoutAmmo` (`KismetMathLibrary.RandomIntegerInRange` 1 30)))
          (:`ShotGunType`
            (set `local.CoutAmmo` (`KismetMathLibrary.RandomIntegerInRange` 1 7)))
          (:`SniperRifle`
            (set `local.CoutAmmo` (`KismetMathLibrary.RandomIntegerInRange` 1 5)))
          (:`GrenadeLauncher`
            (set `local.CoutAmmo` (`KismetMathLibrary.RandomIntegerInRange` 1 2)))))
      (:`then_1`
        (set `/Game/BluePrint/BP_DropActorComponente.Cout` (* (`local.CoutAmmo`) (`self.AmmoDropMult`)) _returnvalue)))))

(fn `MeleeAttack`
  (params (StartTrace :type "Float (double-precision)" :default 50.0) (EndTrace :type "Float (double-precision)" :default 100.0) (Damage :type "Float (double-precision)" :default 50.0) (DamageRafius :type "Float (double-precision)" :default 30.0))
  (returns (Success :type Boolean))
  (bind _returnvalue (`self.K2_GetActorLocation`))
  (bind _returnvalue_2 (`self.GetActorForwardVector`))
  (bind _outhit (`KismetSystemLibrary.SphereTraceSingle` (+ _returnvalue (* _returnvalue_2 StartTrace)) (+ _returnvalue (* _returnvalue_2 EndTrace)) DamageRafius "TraceTypeQuery6" false (`|MakeArray` self :!type "Actor Object Reference") "ForDuration"))
  (bind (_bblockinghit _binitialoverlap _time _distance _location _impactpoint _normal _impactnormal _physmat _hitactor) (`GameplayStatics.BreakHitResult` _outhit))
  (`/Engine/EditorBlueprintResources/StandardMacros.IsValid` _hitactor
    (:`Is Valid`
      (if (`self.ActorHasTag` _hitactor "Player")
        (`GameplayStatics.ApplyDamage` _hitactor Damage (`self.GetController`) self)
        (return true)
        (else
          _)))
    (:`Is Not Valid`
      _))
  (return false))

(fn `PawnCanAttack`
  (returns (bIsCanAttack :type Boolean))
  (return (`self.CanAttack`)))

(fn `PawnCanMove`
  (returns (bIsCanMove :type Boolean))
  (return (`self.CanMove`)))

(fn `SetAttackState`
  (params (CanAttack :type Boolean))
  (set `self.CanAttack` CanAttack))

(fn `SetStateMovement`
  (params (CanMove :type Boolean))
  (set `self.CanMove` CanMove))

(fn `UserConstructionScript`)