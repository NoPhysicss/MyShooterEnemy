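; Base enemy character that handles damage reactions, death and random ammo drops, and takes its kill score from the game mode.
; Damage feeds a health component, whose change event spawns floating damage numbers and rolls for stun, hit montage and slowdown.
; Death unpossesses the pawn, plays a montage, then switches to ragdoll physics and triggers any drop component added at BeginPlay.
; Player-chasing movement nodes are present but disconnected.
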(event `self.ReceiveBeginPlay`
  ;[1 1 1] BeginPlay
  (`self.InitDropComponente`)
  (bind _asbp_game_mode (cast `/Game/BluePrint/Game/BP_GameMode` (`GameplayStatics.GetGameMode`)))
  (set `/Game/BluePrint/BP_KillScoreComponente.Score` (`/Game/BluePrint/Game/BP_GameMode.Enemy Score` _asbp_game_mode) (`self.BP_KillScoreComponente`)))

(event `self.ReceiveTick`
  (params (DeltaSeconds :type "Float (single-precision)"))
  (bind _charactermovement (`self.CharacterMovement`))
  ;[1 1 1] Tick with movement
  (set `self.DeltaTime` DeltaSeconds)
  (if (`self.SlowDownSpeed`)
    (set `CharacterMovementComponent.MaxWalkSpeed` (`KismetMathLibrary.FInterpTo` (`KismetMathLibrary.VSize` (`self.GetVelocity`)) 250.0 (`self.DeltaTime`) 0.1) _charactermovement)
    (else
      (set `CharacterMovementComponent.MaxWalkSpeed` 350.0 _charactermovement))))

(event `self.ReceiveAnyDamage`
  (params (Damage :type "Float (single-precision)") (DamageType :type "DamageType Object Reference") (InstigatedBy :type "Controller Object Reference") (DamageCauser :type "Actor Object Reference"))
  ;[1 1 1] Enemy Take Damaga
  (`MyShooterHealthComponent.ChangeCurrentHealt` (`self.MyShooterHealth`) (* Damage -1.0)))

(event `self.MyShooterHealth.OnHealthChange`
  (params (Health :type "Float (single-precision)") (Damage :type "Float (single-precision)"))
  ;[1 1 1] Enemy Health
  (if (not (`self.IsDead`))
    (if (> (`self.StunChance`) (`KismetMathLibrary.RandomFloat`))
      (`self.Confusiont Enabled`)
      (else
        (`self.Hit Enabled`)))
    (bind _returnvalue (`|SpawnActorFromClass` "/Game/BluePrint/InteractionEnvironment/DamageWidget/DisplayDamageActor.DisplayDamageActor_C" (`KismetMathLibrary.MakeTransform` (+ (`self.K2_GetActorLocation`) (+ (`KismetMathLibrary.MakeVector` (`KismetMathLibrary.RandomFloatInRange` -10.0 10.0) (`KismetMathLibrary.RandomFloatInRange` -10.0 10.0)) (`self.Local Point Spawn Health Number`))) (struct :`Yaw` 180.0)) "Undefined" "MultiplyWithRoot" null null))
    (`/Game/BluePrint/InteractionEnvironment/DamageWidget/DisplayDamageActor.InitActor` _returnvalue Damage Health)
    (if (> (`KismetMathLibrary.RandomFloat`) (`self.SlowDownSpeedChande`))
      (set `self.SlowDownSpeed` true)
      (`KismetSystemLibrary.K2_SetTimerDelegate` (delegate `SlowDownSpeedTimer`)))))

(event `SlowDownSpeedTimer`
  ;[1 1 1] Enemy Health
  (set `self.SlowDownSpeed` false))

(event `self.MyShooterHealth.OnDead`
  (bind _deathanims (`self.DeathAnims`))
  (bind _mesh (`self.Mesh`))
  (bind _capsulecomponent (`self.CapsuleComponent`))
  (bind _dropcomponente (`self.DropComponente`))
  (bind _output (`|GetArrayItem` _deathanims (- (`KismetArrayLibrary.Array_Length` _deathanims) 1)))
  ;[1 1 1] Enemy Dead Event
  (if (not (`self.IsDead`))
    (`self.DeadEvent`)
    (`/Engine/EditorBlueprintResources/StandardMacros.IsValid` _output
      (:`Is Valid`
        (`|PlayMontage` (`self.Mesh`) _output
          (:`then`
            _)
          (:`OnInterrupted`
            _))
        (`PrimitiveComponent.SetCollisionEnabled` _mesh "PhysicsOnly")
        (`PrimitiveComponent.SetCollisionResponseToChannel` _capsulecomponent "ECC_WorldStatic" "ECR_Ignore")
        (`PrimitiveComponent.SetCollisionResponseToChannel` _capsulecomponent "ECC_Pawn" "ECR_Ignore")
        (`PrimitiveComponent.SetCollisionResponseToChannel` _capsulecomponent "ECC_WorldDynamic" "ECR_Ignore")
        (`PrimitiveComponent.SetCollisionResponseToChannel` _capsulecomponent "ECC_GameTraceChannel4" "ECR_Ignore")
        (`PrimitiveComponent.SetCollisionProfileName` _mesh "PhysicsActor" false)
        (`PrimitiveComponent.SetSimulatePhysics` _mesh true)
        (`/Engine/EditorBlueprintResources/StandardMacros.IsValid` _dropcomponente
          (:`Is Valid`
            (`/Game/BluePrint/BP_DropActorComponente.Drop` _dropcomponente)))))))

(fn `Confusiont Disabled Timer`
  (`self.SetStateMovement` true)
  (set `CharacterMovementComponent.MaxWalkSpeed` 500.0 (`self.CharacterMovement`))
  (set `self.bIsConfused` false))

(fn `Confusiont Enabled`
  (locals (StunAnims :type "Array of AnimMontage Object Reference") (CurrentMontage :type "AnimMontage Object Reference"))
  (bind _stunanims (`local.StunAnims`))
  (`self.SetStateMovement` false)
  (bind _output_get (set `local.CurrentMontage` (`|GetArrayItem` _stunanims (`KismetMathLibrary.RandomIntegerInRange` 0 (- (`KismetArrayLibrary.Array_Length` _stunanims) 1)))))
  (`KismetSystemLibrary.K2_SetTimer` null "Confusiont Disabled Timer" (`AnimationAsset.GetPlayLength` _output_get))
  (`self.PlayAnimMontage` (`local.CurrentMontage`))
  (set `CharacterMovementComponent.MaxWalkSpeed` 0.0 (`self.CharacterMovement`))
  (set `self.bIsConfused` true))

(fn `DeadEvent`
  (`Controller.UnPossess` (`self.GetController`))
  (`self.SetLifeSpan` 10.0)
  (`self.SetStateMovement` false)
  (`self.SetAttackState` false)
  (set `self.IsDead` true))

(fn `Hit Enabled`
  (locals (HitAnimChance :type "Float (double-precision)" :default 0.2) (HitAnims :type "Array of AnimMontage Object Reference"))
  (bind _hitanims (`local.HitAnims`))
  (if (`self.bIsConfused`)
    _
    (elif (> (`KismetMathLibrary.RandomFloat`) (`local.HitAnimChance`))
      (`self.PlayAnimMontage` (`|GetArrayItem` _hitanims (`KismetMathLibrary.RandomIntegerInRange` 0 (- (`KismetArrayLibrary.Array_Length` _hitanims) 1)))))))

(fn `InitDropComponente`
  (locals (CoutAmmo :type Integer :default 1))
  (if (< (`KismetMathLibrary.RandomFloat`) 0.33)
    (bind _returnvalue (`AddComponent|NODE_AddBP_DropActorComponente-0`))
    (set `self.DropComponente` _returnvalue)
    (bind _output_get (set `/Game/BluePrint/BP_DropActorComponente.Type` (select `int` (`KismetMathLibrary.RandomIntegerInRange` 0 3) :`0` "RifleType" :`1` "ShotGunType" :`2` "SniperRifle" :`3` "GrenadeLauncher" :!type "EWeaponType Enum") _returnvalue))
    (`|ExecutionSequence`
      (:`then_0`
        (switch `EWeaponType` _output_get
          (:`RifleType`
            (set `local.CoutAmmo` (`KismetMathLibrary.RandomIntegerInRange` 1 30)))
          (:`ShotGunType`
            (set `local.CoutAmmo` (`KismetMathLibrary.RandomIntegerInRange` 1 7)))
          (:`SniperRifle`
            (set `local.CoutAmmo` (`KismetMathLibrary.RandomIntegerInRange` 1 5)))
          (:`GrenadeLauncher`
            (set `local.CoutAmmo` (`KismetMathLibrary.RandomIntegerInRange` 1 2)))))
      (:`then_1`
        (set `/Game/BluePrint/BP_DropActorComponente.Cout` (`local.CoutAmmo`) _returnvalue)))))

(fn `SetAttackState`
  (params (CanAttack :type Boolean))
  (set `self.CanAttack` CanAttack))

(fn `SetStateMovement`
  (params (CanMove :type Boolean))
  (set `self.CanMove` CanMove))

(fn `UserConstructionScript`)