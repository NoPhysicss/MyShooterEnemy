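; Player shooter character that handles movement-state input, a configurable boom camera, shield effects, blood decals and periodic noise reporting.
; Weapon reload and fire events drive ABP_Manny and the inventory HUD, while number keys swap a caught pickup into a slot and drop the old weapon.
; Inventory loads from PlayerState on BeginPlay and saves on unpossess.
; Death ragdolls the body, then requests a GameMode respawn or shows the end-game screen.
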(event `self.ReceiveBeginPlay`
  ;[1 1 1] Begin Play
  (bind _asabp_manny (cast `/Game/BluePrint/Charecter/Mannequins/Animations/ABP_Manny` (`SkeletalMeshComponent.GetAnimInstance` (`self.Mesh`))))
  (set `self.AnimChar` _asabp_manny)
  (bind _returnvalue (`MyShooterHealthComponent.GetMaxHealt` (`self.CharHealthComponent`)))
  (set `self.MaximalHealth` _returnvalue)
  (add `MyShooterHealthComponent.OnShieldChange` (`self.CharHealthComponent`) (`|CreateDelegate` :!event `ShieldChange`))
  (bind _asbp_player_state (cast `/Game/BluePrint/Game/BP_PlayerState` (`Controller.PlayerState` (`GameplayStatics.GetPlayerController` 0))))
  (`MyInventoryComponent.InitInventory` (`self.InventoryComponent`) (`/Game/BluePrint/Game/BP_PlayerState.Weapon Slot` _asbp_player_state) (`/Game/BluePrint/Game/BP_PlayerState.Ammo Slot` _asbp_player_state))
  (bind _asbp_player_controller (cast `/Game/BluePrint/Game/BP_PlayerController` (`GameplayStatics.GetPlayerController` 0)))
  (`/Game/BluePrint/Widget/Inventory/BPW_InventoryStats.InitInventoryStatsWidget` (`/Game/BluePrint/Widget/BPW_InGame.InventoryStatsWidget` (`/Game/BluePrint/Game/BP_PlayerController.InGameWidget` _asbp_player_controller)) self)
  (`KismetSystemLibrary.K2_SetTimerDelegate` (delegate `NoiseEvent`) 1.0 true))

(event `NoiseEvent`
  ;[1 1 1] Begin Play
  (`AISense_Hearing.ReportNoiseEvent` (`self.K2_GetActorLocation`) 1.0 self))

(event `ShieldChange`
  (params (Shield :type "Float (single-precision)") (Damage :type "Float (single-precision)"))
  (bind _mesh (`self.Mesh`))
  (bind _bisalive (`self.bIsAlive`))
  ;[1 1 1] ShieldChange
  (if (<= Shield 0.0)
    (if (`self.ShieldBreak`)
      (if _bisalive
        (`NiagaraComponent.SetAsset` (`self.ShieldEnabling`) "/Game/Basic_VFX/Niagara/NS_Basic_9.NS_Basic_9" true)
        (set `self.ShieldBreak` false)
        (`GameplayStatics.SpawnSoundAttached` "/Game/FX_Effect/ShieldFxes/Breake_Isaac_Cue.Breake_Isaac_Cue" _mesh "None" (0.0 0.0 0.0) (struct) "KeepRelativeOffset" false 1.0 1.0 0.0 null null)
        (`GameplayStatics.SpawnSoundAttached` "/Game/FX_Effect/ShieldFxes/ShieldDown_Cue.ShieldDown_Cue" _mesh "None" (0.0 0.0 0.0) (struct) "KeepRelativeOffset" false 1.0 1.0 0.0 null null)))
    (elif (> Shield 10.0)
      (if (`self.ShieldBreak`)
        _
        (elif _bisalive
          (`NiagaraComponent.SetAsset` (`self.ShieldEnabling`) "/Game/Basic_VFX/Niagara/NS_Basic_16.NS_Basic_16" true)
          (set `self.ShieldBreak` true)
          (`GameplayStatics.SpawnSoundAttached` "/Game/FX_Effect/ShieldFxes/ShieldUp_Cue.ShieldUp_Cue" _mesh "None" (0.0 0.0 0.0) (struct) "KeepRelativeOffset" false 1.0 1.0 0.0 null null))))))

(event `self.WeaponReloadStart_BP`
  (params (Anim :type "AnimMontage Object Reference"))
  ;[1 1 1] Weapon Anims And Weapon Widget Binds
  (`/Game/BluePrint/Charecter/Mannequins/Animations/ABP_Manny.Reload` (`self.AnimChar`) Anim)
  (bind _asbp_player_controller (cast `/Game/BluePrint/Game/BP_PlayerController` (`self.GetController`)))
  (bind _ingamewidget (`/Game/BluePrint/Game/BP_PlayerController.InGameWidget` _asbp_player_controller))
  (`/Engine/EditorBlueprintResources/StandardMacros.IsValid` _ingamewidget
    (:`Is Valid`
      (bind _asbp_my_shooter_character (cast `/Game/BluePrint/Charecter/BP_MyShooterCharacter` (`GameplayStatics.GetPlayerPawn` 0)))
      (bind _asbp_weapon_default (cast `/Game/BluePrint/Weapon/BP_WeaponDefault` (`self.GetCurrentWeapon` _asbp_my_shooter_character)))
      (`/Game/BluePrint/Widget/Inventory/BPW_InventoryStats.WeaponStartReload` (`/Game/BluePrint/Widget/BPW_InGame.InventoryStatsWidget` _ingamewidget) (`self.GetCurrentWeaponIndex`) _asbp_weapon_default))))

(event `self.WeaponReloadEnd_BP`
  (params (bIsSuccess :type Boolean))
  ;[1 1 1] Weapon Anims And Weapon Widget Binds
  (`/Game/BluePrint/Charecter/Mannequins/Animations/ABP_Manny.Reload End` (`self.AnimChar`) bIsSuccess)
  (bind _asbp_player_controller (cast `/Game/BluePrint/Game/BP_PlayerController` (`self.GetController`)))
  (bind _ingamewidget (`/Game/BluePrint/Game/BP_PlayerController.InGameWidget` _asbp_player_controller))
  (`/Engine/EditorBlueprintResources/StandardMacros.IsValid` _ingamewidget
    (:`Is Valid`
      (`/Game/BluePrint/Widget/Inventory/BPW_InventoryStats.WeaponEndReload` (`/Game/BluePrint/Widget/BPW_InGame.InventoryStatsWidget` _ingamewidget) (`self.GetCurrentWeaponIndex`) bIsSuccess))))

(event `self.WeaponFireStart_BP`
  (params (Anim :type "AnimMontage Object Reference"))
  ;[1 1 1] Weapon Anims And Weapon Widget Binds
  (`/Game/BluePrint/Charecter/Mannequins/Animations/ABP_Manny.Fire` (`self.AnimChar`) Anim))

(event `InputAction|Aiming`
  (params (Key :type "Key Structure"))
  ;[1 1 1] Movement State
  (:`Pressed`
    (set `self.AimEnable` true)
    (`self.ChangeMovementState` :!label _label))
  (:`Released`
    (set `self.AimEnable` false)
    (goto _label)))

(event `InputAction|Walking`
  (params (Key :type "Key Structure"))
  ;[1 1 1] Movement State
  (:`Pressed`
    (set `self.WalkEnable` true)
    (goto _label))
  (:`Released`
    (set `self.WalkEnable` false)
    (goto _label)))

(event `InputAction|Runing`
  (params (Key :type "Key Structure"))
  ;[1 1 1] Movement State
  (:`Pressed`
    (set `self.RunEnable` true)
    (goto _label))
  (:`Released`
    (set `self.RunEnable` false)
    (goto _label)))

(event `InputAction|ActionNum1`
  (params (Key :type "Key Structure"))
  (bind _catchpickupweapon (`self.CatchPickUpWeapon`))
  (bind _weaponinfo (`/Game/BluePrint/InteractionEnvironment/PickUpActor_Weapon.WeaponInfo` _catchpickupweapon))
  (bind _nameitem (break `WeaponSlot` _weaponinfo))
  ;[1 1 1] Weapon Switch Grom Ground
  (:`Pressed`
    (set `self.CurrentIndexToSwitch` 0)
    (`/Engine/EditorBlueprintResources/StandardMacros.IsValid` _catchpickupweapon :!label _label_2
      (:`Is Valid`
        (if (> (`self.CurrentIndexToSwitch`) (- (`KismetArrayLibrary.Array_Length` (`MyInventoryComponent.WeaponSlots` (`self.InventoryComponent`))) 1))
          (`KismetSystemLibrary.PrintString` "Error, Not Current Index")
          (else
            (`KismetSystemLibrary.PrintString` (`KismetStringLibrary.Conv_NameToString` _nameitem))
            (if (== _nameitem "None")
              (`KismetSystemLibrary.PrintString` "Error, not correct weapon name")
              (else
                (bind (_dropiteminfo _returnvalue) (`MyInventoryComponent.SwitchWeaponToInventory` (`self.InventoryComponent`) _weaponinfo (`self.CurrentIndexToSwitch`) (`self.Current Index Weapon Char`)))
                (if _returnvalue
                  (`self.DropItem` _dropiteminfo)
                  (`/Game/BluePrint/InteractionEnvironment/PickUpActor.PickUpSuccess` _catchpickupweapon))))))))))

(event `InputAction|ActionNum2`
  (params (Key :type "Key Structure"))
  ;[1 1 1] Weapon Switch Grom Ground
  (:`Pressed`
    (set `self.CurrentIndexToSwitch` 1)
    (goto _label_2)))

(event `StartSwetchWeapon`
  (params (CatchPickUpActor :type "/Game/BluePrint/InteractionEnvironment/PickUpActor_Weapon Object Reference"))
  ;[1 1 1] Weapon Switch Widget
  (bind _returnvalue (`|CreateWidget` "/Game/BluePrint/Widget/Inventory/BPW_SwetchWeapon.BPW_SwetchWeapon_C"))
  (`UserWidget.AddToViewport` _returnvalue 0)
  (set `self.CatchPickUpWeapon` CatchPickUpActor))

(event `InputAction|ActionNum3`
  (params (Key :type "Key Structure"))
  ;[1 1 1] Weapon Switch Grom Ground
  (:`Pressed`
    (set `self.CurrentIndexToSwitch` 2)
    (goto _label_2)))

(event `EndSwitchWeapon`
  ;[1 1 1] Weapon Switch Widget
  (set `self.CatchPickUpWeapon` null))

(event `self.CharDead_BP`
  (bind _returnvalue (`GameplayStatics.GetPlayerController` 0))
  (bind _returnvalue_2 (`self.GetCurrentWeapon`))
  ;[1 1 1] Dead Event
  (`PrimitiveComponent.SetCollisionResponseToChannel` (`self.CapsuleComponent`) "ECC_Pawn" "ECR_Ignore")
  (`PrimitiveComponent.SetCollisionResponseToChannel` (`self.Mesh`) "ECC_Pawn" "ECR_Ignore")
  (`/Engine/EditorBlueprintResources/StandardMacros.IsValid` _returnvalue_2
    (:`Is Valid`
      (`self.SetLifeSpan` _returnvalue_2 5.0))
    (:`Is Not Valid`
      _))
  (`self.SetLifeSpan` 5.0)
  (`self.EnableRagDoll`)
  (bind _asbp_game_mode (cast `/Game/BluePrint/Game/BP_GameMode` (`GameplayStatics.GetGameMode`)))
  (bind _success (`/Game/BluePrint/Game/BP_GameMode.TryToRespawnPlayer` _asbp_game_mode))
  (if _success
    (bind _asbp_player_controller (cast `/Game/BluePrint/Game/BP_PlayerController` (`GameplayStatics.GetPlayerController` 0)))
    (`/Game/BluePrint/Widget/Inventory/BPW_InventoryStats.ReUpdateWeaponSlot` (`/Game/BluePrint/Widget/BPW_InGame.InventoryStatsWidget` (`/Game/BluePrint/Game/BP_PlayerController.InGameWidget` _asbp_player_controller)))
    (else
      (bind _returnvalue_3 (`|CreateWidget` "/Game/BluePrint/Widget/BPW_EndGame.BPW_EndGame_C"))
      (`UserWidget.AddToViewport` _returnvalue_3 0)
      (set `PlayerController.bShowMouseCursor` true _returnvalue)
      (bind _asbp_player_controller_2 (cast `/Game/BluePrint/Game/BP_PlayerController` _returnvalue))
      (set `/Game/BluePrint/Game/BP_PlayerController.IsAlive` (`self.bIsAlive`) _asbp_player_controller_2)
      (`KismetSystemLibrary.Delay` 3.0)
      (`GameplayStatics.SetGamePaused` true))))

(event `InputAxis|CameraWheel`
  (params (AxisValue :type "Float (single-precision)"))
  ;[1 1 1] Camera
  (`self.BCameraInputAxis` AxisValue))

(event `self.ReceiveUnpossessed`
  (params (OldController :type "Controller Object Reference"))
  (bind _inventorycomponent (`self.InventoryComponent`))
  ;[1 1 1] Dead Event
  (bind _asbp_player_state (cast `/Game/BluePrint/Game/BP_PlayerState` (`Controller.PlayerState` OldController)))
  (`/Game/BluePrint/Game/BP_PlayerState.SaveCurrentInventory` _asbp_player_state (`MyInventoryComponent.WeaponSlots` _inventorycomponent) (`MyInventoryComponent.AmmoSlots` _inventorycomponent))
  (bind _asbp_player_controller (cast `/Game/BluePrint/Game/BP_PlayerController` OldController))
  (`/Game/BluePrint/Widget/Inventory/BPW_InventoryStats.UnbindAllEvents` (`/Game/BluePrint/Widget/BPW_InGame.InventoryStatsWidget` (`/Game/BluePrint/Game/BP_PlayerController.InGameWidget` _asbp_player_controller)) self))

(event `self.CharHealthComponent.OnHealthChange`
  (params (Health :type "Float (single-precision)") (Damage :type "Float (single-precision)"))
  ;[1 1 1] Blood Decal Spawn
  (`|ExecutionSequence`
    (:`then_0`
      (if (< Damage 0.0)
        (if (< (`KismetMathLibrary.RandomFloat`) 0.33)
          (`GameplayStatics.SpawnDecalAtLocation` (select `int` (`KismetMathLibrary.RandomIntegerInRange` 0 2) :`0` null :`1` null :`2` null :!type "MaterialInterface Object Reference") (10.0 50.0 50.0) (+ (`self.K2_GetActorLocation`) (`KismetMathLibrary.MakeVector` (`KismetMathLibrary.RandomFloatInRange` -40.0 40.0) (`KismetMathLibrary.RandomFloatInRange` -40.0 40.0) -100.0)) (`KismetMathLibrary.MakeRotator` (`KismetMathLibrary.RandomFloatInRange` 0.0 360.0) -90.0) 15.0))))))

(fn `DropItem`
  (params (DropItemInfo :type "DropItem Structure"))
  (bind _returnvalue (`|SpawnActorFromClass` "/Game/BluePrint/InteractionEnvironment/PickUpActor_Weapon.PickUpActor_Weapon_C" (`KismetMathLibrary.MakeTransform` (+ (`self.K2_GetActorLocation`) (* (`self.GetActorForwardVector`) 100.0))) "AdjustIfPossibleButAlwaysSpawn" "MultiplyWithRoot" null null))
  (`/Game/BluePrint/InteractionEnvironment/PickUpActor.InitActor` _returnvalue DropItemInfo))

(fn `UserConstructionScript`
  (bind _cameraboom (`self.CameraBoom`))
  (set `SpringArmComponent.TargetArmLength` (`self.Hieght`) _cameraboom)
  (`SceneComponent.K2_SetRelativeRotation` _cameraboom (`self.RotatorCamera`) false false)
  (set `SpringArmComponent.bEnableCameraLag` (`self.Flow`) _cameraboom)
  (set `SpringArmComponent.CameraLagSpeed` (`self.CoefSmooth`) _cameraboom))