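; Default weapon projectile Blueprint that leaves short-lived blood decals when it hits flesh.
; On a collision sphere hit, a random roll lets about one in three hits continue, then the physical material is checked for Flesh.
; The decal attaches to the hit component, at the hit bone when one is named, with its location derived from the hit normal and a fixed offset.
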(event `self.BulletCollisionSphere.OnComponentHit`
  (params (HitComponent :type "PrimitiveComponent Object Reference") (OtherActor :type "Actor Object Reference") (OtherComp :type "PrimitiveComponent Object Reference") (NormalImpulse :type "Vector Structure") (Hit :type "HitResult Structure (by ref)"))
  (bind (_bblockinghit _binitialoverlap _time _distance _location _impactpoint _normal _impactnormal _physmat _hitactor _hitcomponent _hitbonename _bonename) (`GameplayStatics.BreakHitResult` Hit))
  (bind _returnvalue (- _normal (0.0 0.0 28.0)))
  (if (< (`KismetMathLibrary.RandomFloat`) 0.33)
    (if (== _physmat "/Game/Materials/Flesh.Flesh")
      (if (!= _bonename "None")
        (`GameplayStatics.SpawnDecalAttached` "/Game/BluePrint/Weapon/Decals/BloodDecal/Blood_Hit_Decal.Blood_Hit_Decal" (30.0 30.0 30.0) _hitcomponent _bonename _returnvalue (struct) "KeepRelativeOffset" 10.0)
        (else
          (`GameplayStatics.SpawnDecalAttached` "/Game/BluePrint/Weapon/Decals/BloodDecal/Blood_Hit_Decal.Blood_Hit_Decal" (30.0 30.0 30.0) _hitcomponent "None" _returnvalue (struct) "KeepRelativeOffset" 10.0))))))

(fn `UserConstructionScript`)